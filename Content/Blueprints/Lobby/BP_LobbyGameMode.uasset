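; Lobby game mode that names joining players and runs the start countdown before travelling to the game map.
; On login it sets each player state's nickname from an incrementing counter.
; A looping one-second timer decrements the remaining time on the lobby game state, then server-travels to the third-person map at zero; cancelling clears it.
; A helper function reports whether every player state is ready.
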(event Custom|CountdownTick
  (bind _asbp_lobby_game_state (Utilities|Casting|CastToBP_LobbyGameState (Game|GetGameState)))
  (bind _output_get (Variables|/Game/Blueprints/Lobby/BP_LobbyGameState.BP_LobbyGameState_C|SetRemainingTime _asbp_lobby_game_state (- (Variables|/Game/Blueprints/Lobby/BP_LobbyGameState.BP_LobbyGameState_C|GetRemainingTime _asbp_lobby_game_state) 1)))
  (if (<= _output_get 0)
    (CallFunction|FinishCountdown)
    (else
      (Development|PrintString (Utilities|String|ToString(Integer) (Variables|/Game/Blueprints/Lobby/BP_LobbyGameState.BP_LobbyGameState_C|GetRemainingTime _asbp_lobby_game_state))))))

(event Custom|CancelCountdown
  (Utilities|Time|ClearandInvalidateTimerbyHandle (Variables|Default|GetCountdownTimerHandle))
  (bind _asbp_lobby_game_state (Utilities|Casting|CastToBP_LobbyGameState (Game|GetGameState)))
  (Variables|/Game/Blueprints/Lobby/BP_LobbyGameState.BP_LobbyGameState_C|SetbCountdownActive _asbp_lobby_game_state false)
  (Variables|/Game/Blueprints/Lobby/BP_LobbyGameState.BP_LobbyGameState_C|SetRemainingTime _asbp_lobby_game_state 0))

(event Custom|StartCountdown
  (bind _asbp_lobby_game_state (Utilities|Casting|CastToBP_LobbyGameState (Game|GetGameState)))
  (if (not (Variables|/Game/Blueprints/Lobby/BP_LobbyGameState.BP_LobbyGameState_C|GetbCountdownActive _asbp_lobby_game_state))
    (Variables|/Game/Blueprints/Lobby/BP_LobbyGameState.BP_LobbyGameState_C|SetbCountdownActive _asbp_lobby_game_state true)
    (Variables|/Game/Blueprints/Lobby/BP_LobbyGameState.BP_LobbyGameState_C|SetRemainingTime _asbp_lobby_game_state 10)
    (bind _returnvalue (Utilities|Time|SetTimerbyEvent (delegate Custom|CountdownTick) 1.0 true))
    (Variables|Default|SetCountdownTimerHandle _returnvalue)))

(event Custom|FinishCountdown
  (Utilities|Time|ClearandInvalidateTimerbyHandle (Variables|Default|GetCountdownTimerHandle))
  (bind _asbp_lobby_game_state (Utilities|Casting|CastToBP_LobbyGameState (Game|GetGameState)))
  (Variables|/Game/Blueprints/Lobby/BP_LobbyGameState.BP_LobbyGameState_C|SetbCountdownActive _asbp_lobby_game_state false)
  (Variables|/Game/Blueprints/Lobby/BP_LobbyGameState.BP_LobbyGameState_C|SetRemainingTime _asbp_lobby_game_state 0)
  (Development|ExecuteConsoleCommand "ServerTravel /Game/Maps/Lvl_ThirdPerson" 0))

(event EventPostLogin
  (params (NewPlayer :type Player%20Controller%20Object%20Reference))
  (bind _asbp_lobby_player_state (Utilities|Casting|CastToBP_LobbyPlayerState (Variables|/Script/Engine.Controller|GetPlayerState NewPlayer)))
  (Variables|/Game/Blueprints/Lobby/BP_LobbyPlayerState.BP_LobbyPlayerState_C|SetNickname _asbp_lobby_player_state (Utilities|String|ToString(Integer) (Variables|Default|GetTest)))
  (Math|Integer|IncrementInt (Variables|Default|GetTest)))

(fn ConstructionScript)

(fn CheckAllPlayersReady
  (LocalVariables|SetbResult true)
  (bind _asbp_lobby_game_state (Utilities|Casting|CastToBP_LobbyGameState (Game|GetGameState)))
  (bind _array_element (Utilities|Array|ForEachLoopwithBreak (Variables|/Script/Engine.GameStateBase|GetPlayerArray _asbp_lobby_game_state) :!label _label)
    (:LoopBody
      (bind _asbp_lobby_player_state (Utilities|Casting|CastToBP_LobbyPlayerState _array_element))
      (if (not (Variables|/Game/Blueprints/Lobby/BP_LobbyPlayerState.BP_LobbyPlayerState_C|GetbIsReady _asbp_lobby_player_state))
        (LocalVariables|SetbResult false)
        (goto _label Break)))
    (:Completed
      (return (LocalVariables|GetbResult)))))