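; Lobby player controller that shows the lobby widget for the local player and relays lobby actions to the server.
; C2S events set the nickname and toggle ready on BP_LobbyPlayerState, then BP_LobbyGameMode starts or cancels the countdown based on all-ready status.
; Kick requests require a local controller and a valid target other than player state 0, but only print authorization.
; IsLobbyHost identifies the host as a locally controlled controller with authority.
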(event Custom|C2S_SetReady
  ;[0.15 0.15 0.15 0.5] 서버에서 실행될 로직 = Replication에 해당됨.
  (bind _asbp_lobby_player_state (Utilities|Casting|CastToBP_LobbyPlayerState (Variables|GetPlayerState self)))
  (Default|SetReadyState _asbp_lobby_player_state (not (Variables|/Game/Blueprints/Lobby/BP_LobbyPlayerState.BP_LobbyPlayerState_C|GetbIsReady _asbp_lobby_player_state)))
  (bind _asbp_lobby_game_mode (Utilities|Casting|CastToBP_LobbyGameMode (Game|GetGameMode)))
  (bind _allready (Default|CheckAllPlayersReady _asbp_lobby_game_mode))
  (if _allready
    (Default|StartCountdown _asbp_lobby_game_mode)
    (else
      (Default|CancelCountdown _asbp_lobby_game_mode))))

(event Custom|C2S_SetNickname
  (params (NewNickname :type String))
  (bind _asbp_lobby_player_state (Utilities|Casting|CastToBP_LobbyPlayerState (Variables|GetPlayerState self)))
  (Variables|/Game/Blueprints/Lobby/BP_LobbyPlayerState.BP_LobbyPlayerState_C|SetNickname _asbp_lobby_player_state NewNickname))

(event Custom|C2S_RequestKick
  (params (TargetPlayerState :type BP%20Lobby%20Player%20State%20Object%20Reference))
  (if (Pawn|IsLocalController)
    (Utilities|IsValid TargetPlayerState
      (:Is%20Valid
        (if (!= (Game|GetPlayerState 0) TargetPlayerState)
          (Development|PrintString "Print String \"Kick Authorized\""))))))

(event EventBeginPlay
  (if (Pawn|IsLocalController)
    (bind _returnvalue (UserInterface|CreateWidget "/Widget/Lobby/WBP_Lobby.WBP_Lobby_C" self))
    (bind _output_get (Variables|Default|SetLobbyWidgetRef _returnvalue))
    (UserInterface|Viewport|AddtoViewport _output_get 0)
    (Variables|Default|SetbShowMouseCursor true)
    (Input|SetInputModeGameandUI self (Variables|Default|GetLobbyWidgetRef) "DoNotLock" true false)))

(fn ConstructionScript)

(fn IsLobbyHost
  (return (and (Ability|HasAuthority) (Pawn|IsLocalController))))