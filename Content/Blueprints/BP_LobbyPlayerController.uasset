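; Lobby player controller that shows the lobby UI and lets the player toggle ready status.
; On BeginPlay, the local controller creates the WBP_Lobby widget, shows the cursor and sets Game and UI input mode.
; Pressing R calls a server RPC, which flips IsReady on BP_LobbyPlayerState through SetReadyState.
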(event Custom|C2S_SetReady
  ;[0.15 0.15 0.15 0.5] 서버에서 실행될 로직 = Replication에 해당됨.
  (Development|PrintString "Server RPC Executed")
  (bind _asbp_lobby_player_state (Utilities|Casting|CastToBP_LobbyPlayerState (Variables|GetPlayerState self)))
  (Default|SetReadyState _asbp_lobby_player_state (not (Variables|/Game/Blueprints/BP_LobbyPlayerState.BP_LobbyPlayerState_C|GetbIsReady _asbp_lobby_player_state))))

(event EventBeginPlay
  (if (Pawn|IsLocalController)
    (bind _returnvalue (UserInterface|CreateWidget "/Widget/Lobby/WBP_Lobby.WBP_Lobby_C" self))
    (bind _output_get (Variables|Default|SetLobbyWidgetRef _returnvalue))
    (UserInterface|Viewport|AddtoViewport _output_get 0)
    (Variables|Default|SetbShowMouseCursor true)
    (Input|SetInputModeGameandUI self (Variables|Default|GetLobbyWidgetRef) "DoNotLock" true false)))

(event Input|KeyboardEvents|R
  (params (Key :type Key%20Structure :default "None"))
  ;[0.15 0.15 0.15 0.5] RPC
  (:Pressed
    (CallFunction|C2SSetReady)))

(fn ConstructionScript)